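; Rhythm game mode that loads a JSON song chart and sets up the Audience mode, then the Doll (Gremlin-side) mode, on successive initialization calls.
; It reads BPM, notes and audio name, loads the SoundWave by soft path, hands sound and notes to the mode, then spawns BP_QuaterNote.
; It precomputes the maximum score using streak multipliers and note-type markers, and sizes the end countdown from the final note.
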(event Custom|calculateHighestScore
  (for _array_element (Variables|Default|GetnoteArray)
    (if (!= (Utilities|String|Len _array_element) 0)
      (Variables|Default|SetnoteCount (+ (Variables|Default|GetnoteCount) 1))
      (if (>= (Variables|Default|GetnoteCount) 30)
        (Variables|Default|Setmultiplier 8)
        (elif (>= (Variables|Default|GetnoteCount) 15)
          (Variables|Default|Setmultiplier 4)
          (elif (>= (Variables|Default|GetnoteCount) 5)
            (Variables|Default|Setmultiplier 2)
            (else
              (Variables|Default|Setmultiplier 1)))))
      (if (and (== (Utilities|String|FindSubstring _array_element "L") -1) (and (== (Utilities|String|FindSubstring _array_element "?") -1) (== (Utilities|String|FindSubstring _array_element "/") -1)))
        (Variables|Default|SethighestPotentialScore (+ (* 1000 (Variables|Default|Getmultiplier)) (Variables|Default|GethighestPotentialScore)))
        (else
          (Variables|Default|SethighestPotentialScore (+ (* 2500 (Variables|Default|Getmultiplier)) (Variables|Default|GethighestPotentialScore))))))))

(event Custom|finalCountdownSetup
  (bind _output_get (Variables|Default|SetfinalNote (Utilities|Array|Get(acopy) (Variables|Default|GetnoteArray) (- (Utilities|Array|Length (Variables|Default|GetnoteArray)) 1))))
  (if (== (Utilities|String|Len _output_get) 1)
    (Variables|Default|SetendCountdown 16)
    (elif (!= (Utilities|String|FindSubstring (Variables|Default|GetfinalNote) "/") -1)
      (Variables|Default|SetendCountdown 20)
      (elif (!= (Utilities|String|FindSubstring (Variables|Default|GetfinalNote) "?") -1)
        (Variables|Default|SetendCountdown 24)
        (elif (!= (Utilities|String|FindSubstring (Variables|Default|GetfinalNote) "L") -1)
          (Variables|Default|SetendCountdown 32)
          (else
            (Variables|Default|SetendCountdown 20)))))))

(fn ConstructionScript)

(fn SplitCool
  (params (str :type String) (delimeter :type String))
  (bind _strarray (Variables|Default|GetstrArray))
  (Variables|Default|SettempStr str)
  (while (.ReturnValue (Utilities|String|Split (Variables|Default|GettempStr) delimeter))
    (Variables|Default|SettempStr (.RightS (Utilities|String|Split (Variables|Default|GettempStr) delimeter)))
    (Utilities|Array|Add _strarray (.LeftS (Utilities|String|Split (Variables|Default|GettempStr) delimeter))))
  (Utilities|Array|Add _strarray (.RightS (Utilities|String|Split (Variables|Default|GettempStr) delimeter)))
  (Utilities|Array|RemoveIndex _strarray (- (Utilities|Array|Length _strarray) 2))
  (return _strarray))

(fn GameInitialization
  (Class|RhythmGameMode|InitializeModeData)
  (Class|RhythmGameMode|CreateAudioImporter)
  (Development|PrintString "Start")
  (if (Variables|Default|GetaudienceInitialized)
    (if (Variables|Default|GetdollInitialized)
      (bind _returnvalue (Class|RhythmGameMode|GetModeData))
      (return _returnvalue)
      (else
        (Variables|Default|SetdollInitialized true)
        (CallFunction|ModeInitialization (Variables|Default|GetdollMode) (Utilities|String|Append (Utilities|String|Replace (Class|BlueprintPathsLibrary|GetProjectFilePath) "/ProjectGroovy.uproject") "/Content/Data/billie_song.json") false "sideGremlin")
        (return (Variables|Default|GetdollMode))))
    (else
      (Development|PrintString "Audience Start")
      (Variables|Default|SetaudienceInitialized true)
      (CallFunction|ModeInitialization (Variables|Default|GetaudienceMode) (Utilities|String|Append (Utilities|String|Replace (Class|BlueprintPathsLibrary|GetProjectFilePath) "/ProjectGroovy.uproject") "/Content/Data/billie_song.json") true "sideAudience")
      (return (Variables|Default|GetaudienceMode)))))

(fn ModeInitialization
  (params (mode :type Key%20Mode%20Data%20Object%20Reference) (fileName :type String) (activeness :type Boolean) (associatedState :type EAllGameStates%20Enum :default "start"))
  (Variables|Default|SetcurrentState associatedState)
  (Variables|Default|SetcurrentMode mode)
  (Development|PrintString "Hello")
  (bind (_outjsonobject _returnvalue) (Class|JsonBlueprintFunctionLibrary|FromFile (Utilities|Struct|MakeFilePath fileName)))
  (if _returnvalue
    (bind _outvalue (|GetJsonField _outjsonobject "BPM"))
    (bind _output_get (Variables|Default|SetBPM _outvalue))
    (Development|PrintString (Utilities|String|ToString(Integer) _output_get))
    (bind _outvalue_2 (|GetJsonField _outjsonobject "Song"))
    (Variables|Default|SetnoteArray _outvalue_2)
    (CallFunction|CalculateHighestScore)
    (bind _outvalue_3 (|GetJsonField _outjsonobject "mp3"))
    (Development|PrintString (Utilities|String|Append "/Game/Songs/" _outvalue_3))
    (if (Utilities|IsValidSoftObjectReference (Class|KismetSystemLibrary|ToSoftObjRef(SoftObjPath) (Utilities|MakeSoftObjectPath (Utilities|String|Append "/Game/Songs/" _outvalue_3))))
      (bind _returnvalue_2 (Utilities|LoadAssetBlocking (Class|KismetSystemLibrary|ToSoftObjRef(SoftObjPath) (Utilities|MakeSoftObjectPath (Utilities|String|Append "/Game/Songs/" _outvalue_3)))))
      (bind _assound_wave (Utilities|Casting|CastToSoundWave _returnvalue_2)
        (:then
          (bind _output_get_2 (Variables|Default|Setsong _assound_wave))
          (bind _returnvalue_3 (Audio|CreateSound2D _output_get_2 1.0 1.0 0.0 0))
          (bind _output_get_3 (Variables|Default|SetplayingSong _returnvalue_3))
          (CallFunction|FinalCountdownSetup)
          (Development|PrintString "Here")
          (Class|KeyModeData|SetMajorAtrributes (Variables|Default|GetcurrentMode) activeness (Variables|Default|GetcurrentState) _output_get_3 (Variables|Default|GetnoteArray))
          (Game|SpawnActorfromClass "/Game/Blueprints/Blueprints/BP_QuaterNote.BP_QuaterNote_C" (Math|Conversions|ToTransform(Vector) (Math|Vector|VectorZero)) "Undefined" "MultiplyWithRoot" 0 0)
          (Development|PrintString (Utilities|String|ToString(Float) (Variables|/Script/ProjectGroovy.KeyModeData|Gethealth (Variables|Default|GetcurrentMode))))
          (Development|PrintString "Wassup"))
        (:CastFailed
          (Development|PrintString "Not a sound Wave")))
      (else
        (Development|PrintString "Not valid lol")
        (Game|QuitGame 0 "Quit" false)))
    (else
      (Development|PrintString "Failed to load JSON file")
      (Game|QuitGame 0 "Quit" false))))