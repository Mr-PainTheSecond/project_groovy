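; BP_Beats is a scrolling beat marker for the rhythm game that triggers song start and game end.
; At BeginPlay it loops until the game mode's audience is initialized, then copies BPM and base movement from BP_NotePad.
; Tick moves it in local space at that speed while GameState is 1 and unpaused.
; Overlapping BP_Notes starts the song on a fixed measure or quits on the final beat; leaving BP_DeletePad destroys it.
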(event Collision|EventActorEndOverlap
  (params (OtherActor :type Actor%20Object%20Reference))
  (Utilities|Casting|CastToBP_DeletePad OtherActor)
  (Actor|DestroyActor))

(event Collision|EventActorBeginOverlap
  (params (OtherActor :type Actor%20Object%20Reference))
  (bind _returnvalue (Actor|GetActorOfClass "/Game/Blueprints/Blueprints/BP_RhythmGameMode.BP_RhythmGameMode_C"))
  (if (Variables|/Game/Blueprints/Blueprints/BP_RhythmGameMode.BP_RhythmGameMode_C|GetsongPlaying _returnvalue)
    (bind _returnvalue_2 (Actor|GetActorOfClass "/Game/Blueprints/Blueprints/BP_RhythmGameMode.BP_RhythmGameMode_C"))
    (if (== (Variables|Default|Getmeasure) (Variables|/Game/Blueprints/Blueprints/BP_RhythmGameMode.BP_RhythmGameMode_C|GetfinalBeat _returnvalue_2))
      (Utilities|Casting|CastToBP_Notes OtherActor)
      (Game|QuitGame 0 "Quit" false))
    (elif (== (Variables|Default|Getmeasure) 24)
      (Utilities|Casting|CastToBP_Notes OtherActor)
      (bind _returnvalue_3 (Actor|GetActorOfClass "/Game/Blueprints/Blueprints/BP_RhythmGameMode.BP_RhythmGameMode_C"))
      (Audio|Components|Audio|Play (Variables|/Script/ProjectGroovy.RhythmGameMode|GetplayingSong _returnvalue_3) 0.0)
      (bind _returnvalue_4 (Actor|GetActorOfClass "/Game/Blueprints/Blueprints/BP_RhythmGameMode.BP_RhythmGameMode_C"))
      (Variables|/Game/Blueprints/Blueprints/BP_RhythmGameMode.BP_RhythmGameMode_C|SetsongPlaying _returnvalue_4 true))))

(event EventBeginPlay
  (bind _returnvalue (Actor|GetActorOfClass "/Game/Blueprints/Blueprints/BP_RhythmGameMode.BP_RhythmGameMode_C"))
  (Variables|Default|Setready (Variables|/Game/Blueprints/Blueprints/BP_RhythmGameMode.BP_RhythmGameMode_C|GetaudienceInitialized _returnvalue))
  (while (not (Variables|Default|Getready))
    (bind _returnvalue_2 (Actor|GetActorOfClass "/Game/Blueprints/Blueprints/BP_RhythmGameMode.BP_RhythmGameMode_C"))
    (Variables|Default|Setready (Variables|/Game/Blueprints/Blueprints/BP_RhythmGameMode.BP_RhythmGameMode_C|GetaudienceInitialized _returnvalue_2)))
  (bind _returnvalue_3 (Actor|GetActorOfClass "/Game/Blueprints/Blueprints/BP_NotePad.BP_NotePad_C"))
  (Variables|Default|SetbaseMovement (Variables|/Game/Blueprints/Blueprints/BP_NotePad.BP_NotePad_C|GetbaseMovement _returnvalue_3))
  (Variables|Default|SetBPM (Variables|/Game/Blueprints/Blueprints/BP_NotePad.BP_NotePad_C|GetBPM _returnvalue_3)))

(event EventTick
  (params (DeltaSeconds :type Float%20%28single-precision%29))
  (bind _returnvalue (Actor|GetActorOfClass "/Game/Blueprints/Blueprints/BP_GroovyBase.BP_GroovyBase_C"))
  (if (== (Variables|/Script/ProjectGroovy.ProjectGroovyBase|GetgameState _returnvalue) 1)
    (bind _returnvalue_2 (Actor|GetActorOfClass "/Game/Blueprints/Blueprints/BP_Player.BP_Player_C"))
    (if (not (Variables|/Game/Blueprints/Blueprints/BP_Player.BP_Player_C|Getpaused _returnvalue_2))
      (Transformation|SetActorLocation (Math|Transform|TransformLocation (Transformation|GetActorTransform) (* DeltaSeconds (* (Variables|Default|GetBPM) (Variables|Default|GetbaseMovement)))) false false))))

(fn ConstructionScript)