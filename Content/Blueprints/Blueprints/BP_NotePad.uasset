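; Scrolling segment of the rhythm game's note track for one game mode, moved at BPM-scaled, frame-independent speed while that mode is active and unpaused.
; On BeginPlay it fills itself with measure bars and notes, choosing note classes from markers in the mode's note list.
; Player overlap spawns the next pad, which continues the shared beat count; delete-pad overlap destroys it.
; An exhausted note list drives the game mode's end-of-song countdown.
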(event Custom|setScale
  ;[0.15 0.15 0.15 0.5] Handles the creations and destruction of this actor
  (Variables|Default|Setscale 0.0))

(event Custom|noteControl
  (bind _modedata (Variables|Default|GetmodeData))
  (bind _modedata_2 (Variables|Default|GetmodeData))
  (bind _modedata_3 (Variables|Default|GetmodeData))
  (bind _notelist (Variables|/Script/ProjectGroovy.KeyModeData|GetnoteList _modedata))
  (bind _noteindex (Variables|/Script/ProjectGroovy.KeyModeData|GetnoteIndex _modedata_3))
  (bind _notelist_2 (Variables|/Script/ProjectGroovy.KeyModeData|GetnoteList _modedata_3))
  (bind _noteindex_2 (Variables|/Script/ProjectGroovy.KeyModeData|GetnoteIndex _modedata_2))
  (bind _output (Utilities|Array|Get(acopy) _notelist_2 _noteindex))
  (bind _returnvalue (Utilities|String|GetSubstring _output 0))
  ;[0.15 0.15 0.15 0.5] If the loop from BeginPlay reaches here, it is gurarantee that we are making a note. This section is in charge of determining what note is being created
  (Variables|Default|SetfullNoteStr _output)
  (if (!= -1 (Utilities|String|FindSubstring _output "/"))
    (Utilities|Array|SetArrayElem _notelist _noteindex_2 _returnvalue)
    (CallFunction|CreateNote "/Game/Blueprints/Blueprints/BP_QuaterNote.BP_QuaterNote_C")
    (elif (!= -1 (Utilities|String|FindSubstring _output "?"))
      (Utilities|Array|SetArrayElem _notelist _noteindex_2 _returnvalue)
      (CallFunction|CreateNote "/Game/Blueprints/Blueprints/BP_HalfNote_.BP_HalfNote__C")
      (elif (!= -1 (Utilities|String|FindSubstring _output "L"))
        (Utilities|Array|SetArrayElem _notelist _noteindex_2 _returnvalue)
        (CallFunction|CreateNote "/Game/Blueprints/Blueprints/BP_WholeNote.BP_WholeNote_C")
        (else
          (CallFunction|CreateNote "/Game/Blueprints/Blueprints/BP_PlayNotes.BP_PlayNotes_C"))))))

(event Custom|endSongProcess
  (bind _returnvalue (Actor|GetActorOfClass "/Game/Blueprints/Blueprints/BP_RhythmGameMode.BP_RhythmGameMode_C"))
  (if (> (Variables|/Game/Blueprints/Blueprints/BP_RhythmGameMode.BP_RhythmGameMode_C|GetendCountdown _returnvalue) 0)
    (bind _output_get (Variables|/Game/Blueprints/Blueprints/BP_RhythmGameMode.BP_RhythmGameMode_C|SetendCountdown _returnvalue (- (Variables|/Game/Blueprints/Blueprints/BP_RhythmGameMode.BP_RhythmGameMode_C|GetendCountdown _returnvalue) 1)))
    (Development|PrintString (Utilities|String|ToString(Integer) _output_get))))

(event Custom|createBar
  (bind _returnvalue (Game|SpawnActorfromClass "/Game/Blueprints/Blueprints/BP_Beats.BP_Beats_C" (Math|Conversions|ToTransform(Vector) (Variables|Default|GetnewBoxPOS)) "Undefined" "MultiplyWithRoot" 0 0))
  (Variables|/Game/Blueprints/Blueprints/BP_Beats.BP_Beats_C|SetassoicatedMode _returnvalue (Variables|Default|GetassociatedState))
  (Variables|Default|SetfirstBarCreated true)
  (Transformation|SetActorRotation _returnvalue (Variables|Default|GetdefaultRotations))
  (Variables|/Game/Blueprints/Blueprints/BP_Beats.BP_Beats_C|Setmeasure _returnvalue (Variables|Default|GetbarCount))
  (bind _returnvalue_2 (Actor|GetActorOfClass "/Game/Blueprints/Blueprints/BP_RhythmGameMode.BP_RhythmGameMode_C"))
  (if (and (<= (Variables|/Game/Blueprints/Blueprints/BP_RhythmGameMode.BP_RhythmGameMode_C|GetendCountdown _returnvalue_2) 0) (== (Variables|/Game/Blueprints/Blueprints/BP_RhythmGameMode.BP_RhythmGameMode_C|GetfinalBeat _returnvalue_2) -1))
    (bind _output_get (Variables|/Game/Blueprints/Blueprints/BP_RhythmGameMode.BP_RhythmGameMode_C|SetfinalBeat _returnvalue_2 (Variables|Default|GetbarCount)))
    (Development|PrintString (Utilities|String|ToString(Integer) _output_get))))

(event Collision|EventActorEndOverlap
  (params (OtherActor :type Actor%20Object%20Reference))
  (Utilities|Casting|CastToBP_DeletePad OtherActor)
  (Actor|DestroyActor))

(event EventBeginPlay
  ;[0.15 0.15 0.15 0.5] Variable Initialization
  (bind _returnvalue (Actor|GetActorOfClass "/Game/Blueprints/Blueprints/BP_RhythmGameMode.BP_RhythmGameMode_C"))
  (bind _output_get (Variables|Default|SetrythmGameRef _returnvalue))
  (bind _modedata (Default|GameInitialization _output_get))
  (bind _output_get_2 (Variables|Default|SetmodeData _modedata))
  (Variables|Default|SetassociatedState (Variables|/Script/ProjectGroovy.KeyModeData|GetgameState _output_get_2))
  (Variables|Default|SetbarCount (Variables|/Script/ProjectGroovy.KeyModeData|GettotalQuarterBeats _output_get_2))
  (Transformation|SetActorRotation (Variables|Default|GetdefaultRotations))
  (if (Variables|/Game/Blueprints/Blueprints/BP_RhythmGameMode.BP_RhythmGameMode_C|GetfirstNotePadCreated (Variables|Default|GetrythmGameRef))
    (if (Variables|/Game/Blueprints/Blueprints/BP_RhythmGameMode.BP_RhythmGameMode_C|GetfirstDollCreated (Variables|Default|GetrythmGameRef))
      _
      (else
        (Class|RhythmGameMode|SwapActiveModes (Variables|Default|GetrythmGameRef))))
    (else
      (Variables|Default|Setfirst true)))
  (Variables|Default|SetBPM (Variables|/Game/Blueprints/Blueprints/BP_RhythmGameMode.BP_RhythmGameMode_C|GetBPM (Variables|Default|GetrythmGameRef)))
  (bind _output_get_3 (Variables|Default|SetstartPOS (Transformation|GetActorLocation)))
  (Variables|Default|Setcollided false)
  (Variables|Default|SetcurrentPOS _output_get_3)
  (Variables|Default|Setframes 0.0)
  (bind _outactors (Actor|GetAllActorsOfClass "BP_NotePad_C"))
  (bind _array_element (Utilities|Array|ForEachLoopwithBreak _outactors :!label _label)
    (:LoopBody
      (if (Variables|BP_NotePad_C|Getspawning _array_element)
        (Variables|Default|SetnewMeasureLocation (Math|Integer|%(Integer) (Math|Integer|Absolute(Integer) (Variables|BP_NotePad_C|GetcubeOffsetScale _array_element)) 100))
        (goto _label Break)))
    (:Completed
      ;[0.15 0.15 0.15 0.5] Creates the measure bars and the notes which will be associated with this notepad
      (bind _boxextent (Collision|GetActorArrayBounds (Utilities|Array|MakeArray self)))
      (Variables|Default|SetouterBound (+ (Variables|Default|GetstartPOS) _boxextent))
      (Variables|Default|SetnewBoxPOS (Math|Transform|TransformLocation (Transformation|GetActorTransform) (* "0.000000,5.000000,0.000000" (Class|KismetSystemLibrary|MakeLiteralInteger (Variables|Default|GetcubeOffsetScale)))))
      (while (< (.Z (Math|Vector|BreakVector (Variables|Default|GetnewBoxPOS))) (+ (.Z (Math|Vector|BreakVector (Variables|Default|GetouterBound))) -3.5e+02))
        (if (== (Math|Integer|%(Integer) (Math|Integer|Absolute(Integer) (Variables|Default|GetcubeOffsetScale)) 100) (Variables|Default|GetnewMeasureLocation))
          (CallFunction|CreateBar))
        (if (< (Variables|Default|GetbarCount) 24)
          (Variables|Default|SetbarCount (+ (Variables|Default|GetbarCount) 1) :!label _label_2)
          (Variables|Default|SetcubeOffsetScale (- (Variables|Default|GetcubeOffsetScale) 25))
          (Variables|Default|SetnewBoxPOS (Math|Transform|TransformLocation (Transformation|GetActorTransform) (* "0.000000,5.000000,0.000000" (Variables|Default|GetcubeOffsetScale))))
          (elif (>= (Variables|/Script/ProjectGroovy.KeyModeData|GetnoteIndex (Variables|Default|GetmodeData)) (Utilities|Array|Length (Variables|/Script/ProjectGroovy.KeyModeData|GetnoteList (Variables|Default|GetmodeData))))
            (CallFunction|EndSongProcess)
            (goto _label_2)
            (elif (== (Utilities|String|Len (Utilities|Array|Get(acopy) (Variables|/Script/ProjectGroovy.KeyModeData|GetnoteList (Variables|Default|GetmodeData)) (Variables|/Script/ProjectGroovy.KeyModeData|GetnoteIndex (Variables|Default|GetmodeData)))) 0)
              (Variables|/Script/ProjectGroovy.KeyModeData|SetnoteIndex (Variables|Default|GetmodeData) (+ (Variables|/Script/ProjectGroovy.KeyModeData|GetnoteIndex (Variables|Default|GetmodeData)) 1))
              (Variables|Default|SetcubeOffsetScale (- (Variables|Default|GetcubeOffsetScale) 25))
              (Variables|Default|SetnewBoxPOS (Math|Transform|TransformLocation (Transformation|GetActorTransform) (* "0.000000,5.000000,0.000000" (Variables|Default|GetcubeOffsetScale))))
              (Variables|Default|SetbarCount (+ (Variables|Default|GetbarCount) 1))
              (else
                (CallFunction|NoteControl))))))
      (bind _returnvalue_2 (Actor|GetActorOfClass "/Game/Blueprints/Blueprints/BP_RhythmGameMode.BP_RhythmGameMode_C"))
      (if (Variables|/Game/Blueprints/Blueprints/BP_RhythmGameMode.BP_RhythmGameMode_C|GetfirstNotePadCreated _returnvalue_2)
        (if (Variables|/Game/Blueprints/Blueprints/BP_RhythmGameMode.BP_RhythmGameMode_C|GetfirstDollCreated (Variables|Default|GetrythmGameRef))
          _
          (else
            (Variables|/Game/Blueprints/Blueprints/BP_RhythmGameMode.BP_RhythmGameMode_C|SetfirstDollCreated (Variables|Default|GetrythmGameRef) true)
            (Class|RhythmGameMode|SwapActiveModes (Variables|Default|GetrythmGameRef))))
        (else
          (Variables|/Game/Blueprints/Blueprints/BP_RhythmGameMode.BP_RhythmGameMode_C|SetfirstNotePadCreated _returnvalue_2 true)))
      (Variables|/Script/ProjectGroovy.KeyModeData|SettotalQuarterBeats (Variables|Default|GetmodeData) (Variables|Default|GetbarCount))
      (Development|PrintString (Utilities|String|Append "FINAL BEAT " (Utilities|String|ToString(Integer) (Variables|Default|GetbarCount))))
      (Development|PrintString (Utilities|String|Append "Final Index is: " (Utilities|String|ToString(Integer) (Variables|/Script/ProjectGroovy.KeyModeData|GetnoteIndex (Variables|Default|GetmodeData))))))))

(event EventTick
  (params (DeltaSeconds :type Float%20%28single-precision%29))
  (bind _returnvalue (Transformation|GetActorTransform))
  (bind _basemovement (Variables|Default|GetbaseMovement))
  (bind _bpm (Variables|Default|GetBPM))
  (bind _returnvalue_2 (* _bpm _basemovement))
  (bind _returnvalue_3 (* DeltaSeconds _returnvalue_2))
  (bind _returnvalue_4 (Math|Transform|TransformLocation _returnvalue _returnvalue_3))
  ;[0.15 0.15 0.15 0.5] Moves note along the screen. Speed dependent on BPM, but independent of FPS
  (bind _returnvalue_5 (Actor|GetActorOfClass "/Game/Blueprints/Blueprints/BP_GroovyBase.BP_GroovyBase_C"))
  (if (== (Variables|/Script/ProjectGroovy.ProjectGroovyBase|GetgameState _returnvalue_5) (Math|Conversions|ToInteger(Byte) (Variables|Default|GetassociatedState)))
    (bind _returnvalue_6 (Actor|GetActorOfClass "/Game/Blueprints/Blueprints/BP_Player.BP_Player_C"))
    (if (not (Variables|/Game/Blueprints/Blueprints/BP_Player.BP_Player_C|Getpaused _returnvalue_6))
      (Transformation|SetActorLocation _returnvalue_4 false false)
      (Variables|Default|SetcurrentPOS _returnvalue_4)
      (Variables|Default|Setframes (+ (Variables|Default|Getframes) (Math|Float|MakeLiteralFloat 1.0))))))

(event Collision|EventActorBeginOverlap
  (params (OtherActor :type Actor%20Object%20Reference))
  ;[0.15 0.15 0.15 0.5] Handles the creations and destruction of this actor
  (Utilities|Casting|CastToBP_Player OtherActor)
  (Variables|Default|Setspawning true)
  (Collision|GetActorArrayBounds (Utilities|Array|MakeArray self))
  (if (Variables|Default|Getfirst)
    (Variables|Default|SetbarNoteOffset -1490)
    (else
      (Variables|Default|SetbarNoteOffset -1507)))
  (bind _returnvalue (Game|SpawnActorfromClass "BP_NotePad_C" (Math|Conversions|ToTransform(Vector) (Math|Transform|TransformLocation (Transformation|GetActorTransform) (* "0.000000,5.000000,0.000000" (Class|KismetSystemLibrary|MakeLiteralInteger (Variables|Default|GetbarNoteOffset))))) "Undefined" "MultiplyWithRoot" 0 0))
  (Transformation|SetActorRotation _returnvalue (Transformation|GetActorRotation))
  (CallFunction|SetScale _returnvalue)
  (bind _returnvalue_2 (Actor|GetActorOfClass "/Game/Widgets/RhythmHUD.RhythmHUD_C"))
  (Default|CalculateRank (Variables|/Game/Widgets/RhythmHUD.RhythmHUD_C|GetHUDRef _returnvalue_2))
  (Development|PrintString (Utilities|String|Append "Spawned by " (Utilities|String|EnumtoString (Variables|Default|GetassociatedState)))))

(fn ConstructionScript)

(fn CreateNote
  (params (noteType :type Actor%20Class%20Reference))
  (bind _returnvalue (Game|SpawnActorfromClass noteType (Math|Conversions|ToTransform(Vector) (Variables|Default|GetnewBoxPOS)) "AlwaysSpawn" "MultiplyWithRoot" 0 0))
  (bind _asbp_quater_note (Utilities|Casting|CastToBP_QuaterNote _returnvalue)
    (:then
      (Variables|/Game/Blueprints/Blueprints/BP_QuaterNote.BP_QuaterNote_C|SetassociatedMode _asbp_quater_note (Variables|Default|GetassociatedState))
      (Variables|/Game/Blueprints/Blueprints/BP_QuaterNote.BP_QuaterNote_C|SetquarterBeat _asbp_quater_note (Variables|Default|GetbarCount))
      (Transformation|SetActorRotation _returnvalue (Variables|Default|GetdefaultRotations) :!label _label)
      (if (or (>= (Variables|Default|GetnotesInMeasure) 4) (!= (Utilities|String|FindSubstring (Variables|Default|GetfullNoteStr) ";") -1))
        (Variables|Default|SetbarCount (+ (Variables|Default|GetbarCount) 1))
        (Variables|Default|SetcubeOffsetScale (- (Variables|Default|GetcubeOffsetScale) 25))
        (Variables|Default|SetnewBoxPOS (Math|Transform|TransformLocation (Transformation|GetActorTransform) (* "0.000000,5.000000,0.000000" (Class|KismetSystemLibrary|MakeLiteralInteger (Variables|Default|GetcubeOffsetScale)))))
        (Variables|Default|SetnotesInMeasure 0)
        (else
          (Variables|Default|SetnotesInMeasure (+ (Variables|Default|GetnotesInMeasure) 1)))))
    (:CastFailed
      (bind _asbp_play_notes (Utilities|Casting|CastToBP_PlayNotes _returnvalue)
        (:then
          (Variables|/Game/Blueprints/Blueprints/BP_PlayNotes.BP_PlayNotes_C|SetassociatedMode _asbp_play_notes (Variables|Default|GetassociatedState))
          (goto _label))
        (:CastFailed
          (Development|PrintString "Spawn Went Wrong :(")
          (Game|QuitGame 0 "Quit" false))))))