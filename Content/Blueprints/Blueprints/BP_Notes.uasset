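; BP_Notes is a Blueprint that fills an AllLights collection with references to colored lights.
; On BeginPlay it adds the yellow, blue, green and red lights in sequence, then adds the green light a second time.
; Nothing in it reads the collection afterward, and the construction script is empty.
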(event EventBeginPlay
  (Utilities|Array|Add (Variables|Default|GetallLights) (Variables|Default|Getyellow_light))
  (Utilities|Array|Add (Variables|Default|GetallLights) (Variables|Default|Getblue_light))
  (Utilities|Array|Add (Variables|Default|GetallLights) (Variables|Default|Getgreen_light))
  (Utilities|Array|Add (Variables|Default|GetallLights) (Variables|Default|Getred_light))
  (Utilities|Array|Add (Variables|Default|GetallLights) (Variables|Default|Getgreen_light)))

(fn ConstructionScript)