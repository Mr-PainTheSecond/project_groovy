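; A single rhythm-game note that takes its lane and color from the mode's note list on spawn.
; It moves at a frame-rate-independent, BPM-scaled speed while its mode is current and the player isn't paused.
; The early hitbox activates it; NoteScore grades player key presses by the first overlapped actor in a per-mode hitbox array.
; Leaving BP_Notes while active resets the streak as a miss, and leaving BP_DeletePad destroys it.
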(event Custom|setCollisions
  ;[0.15 0.15 0.15 0.5] Creates an array which stores all the actors that are responsible for determining scoring when a note is played
  (if (== (Variables|Default|GetassociatedMode) (Math|Conversions|ToInteger(Byte) (Utilities|Enum|LiteralenumEAllGameStates "sideAudience")))
    (Variables|Default|SetcollisonIndex 0)
    (else
      (Variables|Default|SetcollisonIndex 1)))
  (bind _outactors (Actor|GetAllActorsOfClass "/Game/Blueprints/Blueprints/BP_Notes.BP_Notes_C"))
  (Variables|Default|SetallNoteScoreActors (Utilities|Array|MakeArray (Utilities|Array|Get(acopy) _outactors (Variables|Default|GetcollisonIndex))))
  (bind _outactors_2 (Actor|GetAllActorsOfClass "/Game/Blueprints/Blueprints/BP_GreatHitbox.BP_GreatHitbox_C"))
  (Utilities|Array|Add (Variables|Default|GetallNoteScoreActors) (Utilities|Array|Get(acopy) _outactors_2 (Variables|Default|GetcollisonIndex)))
  (bind _outactors_3 (Actor|GetAllActorsOfClass "/Game/Blueprints/Blueprints/BP_GoodHitbox.BP_GoodHitbox_C"))
  (Utilities|Array|Add (Variables|Default|GetallNoteScoreActors) (Utilities|Array|Get(acopy) _outactors_3 (Variables|Default|GetcollisonIndex)))
  (bind _outactors_4 (Actor|GetAllActorsOfClass "/Game/Blueprints/Blueprints/BP_OKHitbox.BP_OKHitbox_C"))
  (Utilities|Array|Add (Variables|Default|GetallNoteScoreActors) (Utilities|Array|Get(acopy) _outactors_4 (Variables|Default|GetcollisonIndex)))
  (bind _outactors_5 (Actor|GetAllActorsOfClass "/Game/Blueprints/Blueprints/BP_EarlyHitbox.BP_EarlyHitbox_C"))
  (Utilities|Array|Add (Variables|Default|GetallNoteScoreActors) (Utilities|Array|Get(acopy) _outactors_5 (Variables|Default|GetcollisonIndex)))
  (bind _outactors_6 (Actor|GetAllActorsOfClass "/Game/Blueprints/Blueprints/BP_LateHitbox.BP_LateHitbox_C"))
  (Utilities|Array|Add (Variables|Default|GetallNoteScoreActors) (Utilities|Array|Get(acopy) _outactors_6 (Variables|Default|GetcollisonIndex))))

(event Collision|EventActorEndOverlap
  (params (OtherActor :type Actor%20Object%20Reference))
  ;[0.15 0.15 0.15 0.5] Destroys note after it goes below level geometry
  (Utilities|Casting|CastToBP_DeletePad OtherActor
    (:then
      (Utilities|Array|RemoveItem (Variables|/Script/ProjectGroovy.KeyModeData|GetbeingPlayed (Variables|Default|GetmodeData)) self)
      (Actor|DestroyActor))
    (:CastFailed
      ;[0.15 0.15 0.15 0.5] Note has left all playable hitboxes without being played first, so it is a miss.
      (Utilities|Casting|CastToBP_Notes OtherActor)
      (if (Variables|Default|Getactive)
        (Variables|Default|Setactive false)
        (bind _returnvalue (Actor|GetActorOfClass "/Game/Widgets/RhythmHUD.RhythmHUD_C"))
        (Default|ResetStreak (Variables|/Game/Widgets/RhythmHUD.RhythmHUD_C|GetHUDRef _returnvalue))
        (Class|KeyModeData|RemoveNote (Variables|Default|GetmodeData) self)))))

(event Collision|EventActorBeginOverlap
  (params (OtherActor :type Actor%20Object%20Reference))
  (Utilities|Casting|CastToBP_EarlyHitbox OtherActor)
  (Variables|Default|Setactive true))

(event EventNoteScore
  ;[0.15 0.15 0.15 0.5] Comes from the player class, which has read that the player has pressed a keyboard, so this method will see if it is relevant to this instance of the note, and what to do if it is.
  (bind _returnvalue (Actor|GetActorOfClass "/Game/Blueprints/Blueprints/BP_Player.BP_Player_C"))
  (bind (_array_element _array_index) (Utilities|Array|ForEachLoopwithBreak (Variables|Default|GetallNoteScoreActors) :!label _label)
    (:LoopBody
      (if (Collision|IsOverlappingActor _array_element :!class /Script/Engine.Actor)
        (Variables|Default|Setactive false)
        (bind _returnvalue_2 (Actor|GetActorOfClass "/Game/Widgets/RhythmHUD.RhythmHUD_C"))
        (if (Utilities|Enum|Equal(Enum) (Class|KismetInputLibrary|KeyGetDisplayName (Variables|/Game/Blueprints/Blueprints/BP_Player.BP_Player_C|GetkeyPressed _returnvalue) true) (Class|KismetInputLibrary|KeyGetDisplayName (Utilities|Array|Get(acopy) (Utilities|Array|MakeArray (Variables|Default|GetyellowKey) (Variables|Default|GetblueKey) (Variables|Default|GetgreenKey) (Variables|Default|GetredKey)) (Variables|Default|GetnoteIndex)) true))
          (Development|PrintString (Utilities|Array|Get(acopy) (Variables|Default|GetscoreMessages) _array_index))
          (Default|UpdateScore (Variables|/Game/Widgets/RhythmHUD.RhythmHUD_C|GetHUDRef _returnvalue_2) (Utilities|Array|Get(acopy) (Variables|Default|GetscoreMessages) _array_index) self true)
          (goto _label Break)
          (else
            (Default|UpdateScore (Variables|/Game/Widgets/RhythmHUD.RhythmHUD_C|GetHUDRef _returnvalue_2) "Wrong Note Played" self true)
            (goto _label Break)))))
    (:Completed
      (if (Variables|Default|Getactive)
        (Development|PrintString "Tried to score, but found nothing relevant")))))

(event EventBeginPlay
  (bind _returnvalue (Transformation|GetActorTransform))
  (bind _returnvalue_2 (Math|Transform|TransformLocation _returnvalue "0, 0, 0"))
  (bind (_x _y _z) (Math|Vector|BreakVector _returnvalue_2))
  ;[0.15 0.15 0.15 0.5] Variable Initialization
  (bind _returnvalue_3 (Actor|GetActorOfClass "/Game/Blueprints/Blueprints/BP_RhythmGameMode.BP_RhythmGameMode_C"))
  (bind _returnvalue_4 (Class|RhythmGameMode|GetModeData _returnvalue_3))
  (Variables|Default|SetmodeData _returnvalue_4)
  (Variables|Default|Setready (Variables|/Game/Blueprints/Blueprints/BP_RhythmGameMode.BP_RhythmGameMode_C|GetaudienceInitialized _returnvalue_3))
  (while (not (Variables|Default|Getready))
    (bind _returnvalue_5 (Actor|GetActorOfClass "/Game/Blueprints/Blueprints/BP_RhythmGameMode.BP_RhythmGameMode_C"))
    (Variables|Default|Setready (Variables|/Game/Blueprints/Blueprints/BP_RhythmGameMode.BP_RhythmGameMode_C|GetaudienceInitialized _returnvalue_5)))
  (bind _returnvalue_6 (Actor|GetActorOfClass "/Game/Blueprints/Blueprints/BP_NotePad.BP_NotePad_C"))
  (Variables|Default|SetnoteIndex (Math|Conversions|ToInteger(Byte) (Utilities|Array|Get(acopy) (Variables|/Script/ProjectGroovy.KeyModeData|GetnoteList (Variables|Default|GetmodeData)) (Variables|/Script/ProjectGroovy.KeyModeData|GetnoteIndex (Variables|Default|GetmodeData)))))
  (Variables|/Script/ProjectGroovy.KeyModeData|SetnoteIndex (Variables|Default|GetmodeData) (+ 1 (Variables|/Script/ProjectGroovy.KeyModeData|GetnoteIndex (Variables|Default|GetmodeData))))
  (Variables|Default|SetbaseMovement (Variables|/Game/Blueprints/Blueprints/BP_NotePad.BP_NotePad_C|GetbaseMovement _returnvalue_6))
  (Variables|Default|SetBPM (Variables|/Game/Blueprints/Blueprints/BP_NotePad.BP_NotePad_C|GetBPM _returnvalue_6))
  ;[0.05098 0.05098 0.05098] Sets up the positions and colors for the notes
  (bind _boxextent (Collision|GetActorArrayBounds (Utilities|Array|MakeArray self)))
  (Rendering|Material|SetMaterial (Variables|Default|GetStaticMesh) 0 (Utilities|Array|Get(acopy) (Utilities|Array|MakeArray (Variables|Default|Getyellow) (Variables|Default|Getblue) (Variables|Default|Getgreen) (Variables|Default|Getred)) (Variables|Default|GetnoteIndex)))
  (Transformation|SetActorLocation (Math|Vector|MakeVector _x (.Y (Math|Vector|BreakVector (Math|Transform|TransformLocation _returnvalue (* (Math|Vector|MakeVector 0.0 (.Y (Math|Vector|BreakVector _boxextent)) 0.0) (Utilities|Array|Get(acopy) (Utilities|Array|MakeArray (Math|Float|MakeLiteralFloat 0.0) 2.5 5.0 7.5) (Variables|Default|GetnoteIndex)))))) _z) false false))

(event EventTick
  (params (DeltaSeconds :type Float%20%28single-precision%29))
  ;[0.15 0.15 0.15 0.5] Moves note along the screen. Speed dependent on BPM, but independent of FPS
  (bind _returnvalue (Actor|GetActorOfClass "/Game/Blueprints/Blueprints/BP_GroovyBase.BP_GroovyBase_C"))
  (if (== (Variables|/Script/ProjectGroovy.ProjectGroovyBase|GetgameState _returnvalue) (Math|Conversions|ToInteger(Byte) (Variables|Default|GetassociatedMode)))
    (bind _returnvalue_2 (Actor|GetActorOfClass "/Game/Blueprints/Blueprints/BP_Player.BP_Player_C"))
    (if (not (Variables|/Game/Blueprints/Blueprints/BP_Player.BP_Player_C|Getpaused _returnvalue_2))
      (Transformation|SetActorLocation (Math|Transform|TransformLocation (Transformation|GetActorTransform) (* DeltaSeconds (* (Variables|/Script/ProjectGroovy.KeyModeData|GetBPM (Variables|Default|GetmodeData)) (Variables|Default|GetbaseMovement)))) false false))))

(fn ConstructionScript)