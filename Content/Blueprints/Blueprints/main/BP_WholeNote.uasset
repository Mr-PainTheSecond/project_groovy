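; BP_WholeNote is a whole-note actor for a rhythm game that configures its color and lane when it spawns.
; On BeginPlay it takes its note index from the BP_RhythmGameMode mode data's note list, advances that list's index, and caches BPM and base movement.
; The note index selects both mesh materials and a sideways offset scaled from the actor's bounds.
; It has no movement or overlap logic of its own.
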(event Collision|EventActorBeginOverlap
  (params (OtherActor :type Actor%20Object%20Reference))
  ;[0.05098 0.05098 0.05098] Sets up the positions and colors for the notes
)

(event EventTick
  (params (DeltaSeconds :type Float%20%28single-precision%29)))

(event EventBeginPlay
  (bind _returnvalue (Transformation|GetActorTransform))
  (bind _returnvalue_2 (Math|Transform|TransformLocation _returnvalue "0, 0, 0"))
  (bind (_x _y _z) (Math|Vector|BreakVector _returnvalue_2))
  ;[0.15 0.15 0.15 0.5] Variable Initialization
  (bind _returnvalue_3 (Actor|GetActorOfClass "/Game/Blueprints/Blueprints/main/BP_RhythmGameMode.BP_RhythmGameMode_C"))
  (bind _output_get (Variables|Default|SetrhythmGameRef _returnvalue_3))
  (bind _returnvalue_4 (Class|RhythmGameMode|GetModeData _output_get))
  (Variables|Default|SetmodeData _returnvalue_4)
  (Variables|Default|SetnoteIndex (Math|Conversions|ToInteger(Byte) (Utilities|Array|Get(acopy) (Variables|/Script/ProjectGroovy.KeyModeData|GetnoteList (Variables|Default|GetmodeData)) (Variables|/Script/ProjectGroovy.KeyModeData|GetnoteIndex (Variables|Default|GetmodeData)))))
  (Variables|/Script/ProjectGroovy.KeyModeData|SetnoteIndex (Variables|Default|GetmodeData) (+ (Variables|/Script/ProjectGroovy.KeyModeData|GetnoteIndex (Variables|Default|GetmodeData)) 1))
  (Variables|Default|SetbaseMovement (Variables|/Game/Blueprints/Blueprints/main/BP_RhythmGameMode.BP_RhythmGameMode_C|GetbaseMovement (Variables|Default|GetrhythmGameRef)))
  (Variables|Default|SetBPM (Variables|/Script/ProjectGroovy.KeyModeData|GetBPM (Variables|Default|GetmodeData)))
  ;[0.05098 0.05098 0.05098] Sets up the positions and colors for the notes
  (bind _boxextent (Collision|GetActorArrayBounds (Utilities|Array|MakeArray self)))
  (Rendering|Material|SetMaterial (Variables|Default|GetStaticMesh) 0 (Utilities|Array|Get(acopy) (Utilities|Array|MakeArray (Variables|Default|Getyellow) (Variables|Default|Getblue) (Variables|Default|Getgreen) (Variables|Default|Getred)) (Variables|Default|GetnoteIndex)))
  (Rendering|Material|SetMaterial (Variables|Default|Getm&mCylinder) 0 (Utilities|Array|Get(acopy) (Variables|Default|GetmaterialGirls) (Variables|Default|GetnoteIndex)))
  (Transformation|SetActorLocation (Math|Vector|MakeVector _x (.Y (Math|Vector|BreakVector (Math|Transform|TransformLocation _returnvalue (* (Math|Vector|MakeVector 0.0 (.Y (Math|Vector|BreakVector _boxextent)) 0.0) (Utilities|Array|Get(acopy) (Utilities|Array|MakeArray (Math|Float|MakeLiteralFloat 0.0) 0.043 0.086 0.129) (Variables|Default|GetnoteIndex)))))) _z) false false))

(fn ConstructionScript)