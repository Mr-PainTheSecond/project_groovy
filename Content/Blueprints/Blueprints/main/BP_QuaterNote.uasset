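; Quarter note actor for a rhythm game that takes its lane, color and key from the game mode's note list.
; Tick moves it at BPM-scaled speed while its game state is active and unpaused.
; NoteScore grades start and end against timing hitboxes and the pressed key, reporting to RhythmHUD.
; Overlaps award held-note checkpoints, reset the streak on misses, give last-doll bonuses and destroy it past the delete pad.
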(event OnComponentEndOverlap(mainNote)
  (params (OverlappedComponent :type Primitive%20Component%20Object%20Reference) (OtherActor :type Actor%20Object%20Reference) (OtherComp :type Primitive%20Component%20Object%20Reference) (OtherBodyIndex :type Integer))
  (Utilities|Casting|CastToBP_LateHitbox OtherActor)
  (if (Variables|Default|Getactive)
    (Variables|Default|Setactive false)
    (Development|PrintString "Missed Note")
    (bind _returnvalue (Actor|GetActorOfClass "/Game/Widgets/main/RhythmHUD.RhythmHUD_C"))
    (Default|ResetStreak (Variables|/Game/Widgets/main/RhythmHUD.RhythmHUD_C|GetHUDRef _returnvalue))
    (Class|KeyModeData|RemoveNote (Variables|Default|GetmodeData) self)))

(event OnComponentBeginOverlap(checkpoint_one)
  (params (OverlappedComponent :type Primitive%20Component%20Object%20Reference) (OtherActor :type Actor%20Object%20Reference) (OtherComp :type Primitive%20Component%20Object%20Reference) (OtherBodyIndex :type Integer) (bFromSweep :type Boolean) (SweepResult :type Hit%20Result%20Structure%20%28by%20ref%29))
  (Utilities|Casting|CastToBP_Notes OtherActor)
  (bind _returnvalue (Actor|GetActorOfClass "/Game/Widgets/main/RhythmHUD.RhythmHUD_C"))
  (if (Variables|Default|GetbeingPlayed)
    (Default|CheckpointAward (Variables|/Game/Widgets/main/RhythmHUD.RhythmHUD_C|GetHUDRef _returnvalue))))

(event OnComponentBeginOverlap(checkpoint_two)
  (params (OverlappedComponent :type Primitive%20Component%20Object%20Reference) (OtherActor :type Actor%20Object%20Reference) (OtherComp :type Primitive%20Component%20Object%20Reference) (OtherBodyIndex :type Integer) (bFromSweep :type Boolean) (SweepResult :type Hit%20Result%20Structure%20%28by%20ref%29))
  (Utilities|Casting|CastToBP_Notes OtherActor)
  (bind _returnvalue (Actor|GetActorOfClass "/Game/Widgets/main/RhythmHUD.RhythmHUD_C"))
  (if (Variables|Default|GetbeingPlayed)
    (Default|CheckpointAward (Variables|/Game/Widgets/main/RhythmHUD.RhythmHUD_C|GetHUDRef _returnvalue))))

(event OnComponentEndOverlap(note_complete)
  (params (OverlappedComponent :type Primitive%20Component%20Object%20Reference) (OtherActor :type Actor%20Object%20Reference) (OtherComp :type Primitive%20Component%20Object%20Reference) (OtherBodyIndex :type Integer))
  (Utilities|Casting|CastToBP_Notes OtherActor)
  (if (Variables|Default|GetlastDoll)
    (bind _returnvalue (Actor|GetActorOfClass "/Game/Blueprints/Blueprints/main/BP_GroovyBase.BP_GroovyBase_C"))
    (Variables|/Script/ProjectGroovy.ProjectGroovyBase|SetdollComplete _returnvalue true)
    (bind _returnvalue_2 (Actor|GetActorOfClass "/Game/Widgets/main/RhythmHUD.RhythmHUD_C"))
    (Variables|/Game/Widgets/main/WB_Score.WB_Score_C|Setscore (Variables|/Game/Widgets/main/RhythmHUD.RhythmHUD_C|GetHUDRef _returnvalue_2) (+ (Variables|/Game/Widgets/main/WB_Score.WB_Score_C|Getscore (Variables|/Game/Widgets/main/RhythmHUD.RhythmHUD_C|GetHUDRef _returnvalue_2)) (* (Variables|/Script/ProjectGroovy.ProjectGroovyBase|GetscoreByDoll _returnvalue) 2)))
    (Development|PrintString "Doll Complete")))

(event OnComponentBeginOverlap(note_complete)
  (params (OverlappedComponent :type Primitive%20Component%20Object%20Reference) (OtherActor :type Actor%20Object%20Reference) (OtherComp :type Primitive%20Component%20Object%20Reference) (OtherBodyIndex :type Integer) (bFromSweep :type Boolean) (SweepResult :type Hit%20Result%20Structure%20%28by%20ref%29))
  (Utilities|Casting|CastToBP_OKHitbox OtherActor)
  (Variables|Default|SetcanLetGo true))

(event Custom|setCollisions
  ;[0.15 0.15 0.15 0.5] Creates an array which stores all the actors that are responsible for determining scoring when a note is played
  (if (== (Variables|Default|GetassociatedMode) (Math|Conversions|ToInteger(Byte) (Utilities|Enum|LiteralenumEAllGameStates "sideAudience")))
    (Variables|Default|SetcollisionIndex 0)
    (else
      (Variables|Default|SetcollisionIndex 1)))
  (bind _outactors (Actor|GetAllActorsOfClass "/Game/Blueprints/Blueprints/main/BP_Notes.BP_Notes_C"))
  (Variables|Default|SetallNoteScoreActors (Utilities|Array|MakeArray (Utilities|Array|Get(acopy) _outactors (Variables|Default|GetcollisionIndex))))
  (bind _outactors_2 (Actor|GetAllActorsOfClass "/Game/Blueprints/Blueprints/main/BP_GreatHitbox.BP_GreatHitbox_C"))
  (Utilities|Array|Add (Variables|Default|GetallNoteScoreActors) (Utilities|Array|Get(acopy) _outactors_2 (Variables|Default|GetcollisionIndex)))
  (bind _outactors_3 (Actor|GetAllActorsOfClass "/Game/Blueprints/Blueprints/main/BP_GoodHitbox.BP_GoodHitbox_C"))
  (Utilities|Array|Add (Variables|Default|GetallNoteScoreActors) (Utilities|Array|Get(acopy) _outactors_3 (Variables|Default|GetcollisionIndex)))
  (bind _outactors_4 (Actor|GetAllActorsOfClass "/Game/Blueprints/Blueprints/main/BP_OKHitbox.BP_OKHitbox_C"))
  (Utilities|Array|Add (Variables|Default|GetallNoteScoreActors) (Utilities|Array|Get(acopy) _outactors_4 (Variables|Default|GetcollisionIndex)))
  (bind _outactors_5 (Actor|GetAllActorsOfClass "/Game/Blueprints/Blueprints/main/BP_EarlyHitbox.BP_EarlyHitbox_C"))
  (Utilities|Array|Add (Variables|Default|GetallNoteScoreActors) (Utilities|Array|Get(acopy) _outactors_5 (Variables|Default|GetcollisionIndex)))
  (bind _outactors_6 (Actor|GetAllActorsOfClass "/Game/Blueprints/Blueprints/main/BP_LateHitbox.BP_LateHitbox_C"))
  (Utilities|Array|Add (Variables|Default|GetallNoteScoreActors) (Utilities|Array|Get(acopy) _outactors_6 (Variables|Default|GetcollisionIndex)))
  (bind _outactors_7 (Actor|GetAllActorsOfClass "/Game/Blueprints/Blueprints/main/BP_Great_After.BP_Great_After_C"))
  (Utilities|Array|Add (Variables|Default|GetallNoteScoreActors) (Utilities|Array|Get(acopy) _outactors_7 (Variables|Default|GetcollisionIndex))))

(event Collision|EventActorEndOverlap
  (params (OtherActor :type Actor%20Object%20Reference))
  ;[0.15 0.15 0.15 0.5] Destroys note after it goes below level geometry
  (Utilities|Casting|CastToBP_DeletePad OtherActor)
  (Utilities|Array|RemoveItem (Variables|/Script/ProjectGroovy.KeyModeData|GetbeingPlayed (Variables|Default|GetmodeData)) self)
  (Actor|DestroyActor))

(event EventBeginPlay
  (bind _returnvalue (Transformation|GetActorTransform))
  (bind _returnvalue_2 (Math|Transform|TransformLocation _returnvalue "0, 0, 0"))
  (bind (_x _y _z) (Math|Vector|BreakVector _returnvalue_2))
  ;[0.15 0.15 0.15 0.5] Variable Initialization
  (bind _returnvalue_3 (Actor|GetActorOfClass "/Game/Blueprints/Blueprints/main/BP_RhythmGameMode.BP_RhythmGameMode_C"))
  (bind _output_get (Variables|Default|SetrhythmGameRef _returnvalue_3))
  (bind _returnvalue_4 (Class|RhythmGameMode|GetModeData _output_get))
  (Variables|Default|SetmodeData _returnvalue_4)
  (Actor|GetActorOfClass "/Game/Blueprints/Blueprints/main/BP_RhythmGameMode.BP_RhythmGameMode_C")
  (Variables|Default|SetnoteIndex (Math|Conversions|ToInteger(Byte) (Utilities|Array|Get(acopy) (Variables|/Script/ProjectGroovy.KeyModeData|GetnoteList (Variables|Default|GetmodeData)) (Variables|/Script/ProjectGroovy.KeyModeData|GetnoteIndex (Variables|Default|GetmodeData)))))
  (Variables|/Script/ProjectGroovy.KeyModeData|SetnoteIndex (Variables|Default|GetmodeData) (+ (Variables|/Script/ProjectGroovy.KeyModeData|GetnoteIndex (Variables|Default|GetmodeData)) 1))
  (Variables|Default|SetbaseMovement (Variables|/Game/Blueprints/Blueprints/main/BP_RhythmGameMode.BP_RhythmGameMode_C|GetbaseMovement (Variables|Default|GetrhythmGameRef)))
  (Variables|Default|SetBPM (Variables|/Script/ProjectGroovy.KeyModeData|GetBPM (Variables|Default|GetmodeData)))
  ;[0.05098 0.05098 0.05098] Sets up the positions and colors for the notes
  (bind _boxextent (Collision|GetActorArrayBounds (Utilities|Array|MakeArray self)))
  (Rendering|Material|SetMaterial (Variables|Default|GetStaticMesh) 0 (Utilities|Array|Get(acopy) (Utilities|Array|MakeArray (Variables|Default|Getyellow) (Variables|Default|Getblue) (Variables|Default|Getgreen) (Variables|Default|Getred)) (Variables|Default|GetnoteIndex)))
  (Rendering|Material|SetMaterial (Variables|Default|Getm&mCylinder) 0 (Utilities|Array|Get(acopy) (Variables|Default|GetmaterialGirls) (Variables|Default|GetnoteIndex)))
  (Transformation|SetActorLocation (Math|Vector|MakeVector _x (.Y (Math|Vector|BreakVector (Math|Transform|TransformLocation _returnvalue (* (Math|Vector|MakeVector 0.0 (.Y (Math|Vector|BreakVector _boxextent)) 0.0) (Utilities|Array|Get(acopy) (Utilities|Array|MakeArray (Math|Float|MakeLiteralFloat 0.0) 0.185 0.37 0.555) (Variables|Default|GetnoteIndex)))))) _z) false false)
  (Variables|Default|SetnoteKey (Utilities|Array|Get(acopy) (Utilities|Array|MakeArray (Variables|Default|Getyellow_key) (Variables|Default|Getblue_key) (Variables|Default|Getgreen_key) (Variables|Default|Getred_key)) (Variables|Default|GetnoteIndex)))
  (Variables|Default|Setactive true))

(event EventTick
  (params (DeltaSeconds :type Float%20%28single-precision%29))
  ;[0.15 0.15 0.15 0.5] Moves note along the screen. Speed dependent on BPM, but independent of FPS
  (bind _returnvalue (Actor|GetActorOfClass "/Game/Blueprints/Blueprints/main/BP_GroovyBase.BP_GroovyBase_C"))
  (if (== (Variables|/Script/ProjectGroovy.ProjectGroovyBase|GetgameState _returnvalue) (Math|Conversions|ToInteger(Byte) (Variables|Default|GetassociatedMode)))
    (bind _returnvalue_2 (Actor|GetActorOfClass "/Game/Blueprints/Blueprints/main/BP_Player.BP_Player_C"))
    (if (not (Variables|/Game/Blueprints/Blueprints/main/BP_Player.BP_Player_C|Getpaused _returnvalue_2))
      (Transformation|SetActorLocation (Math|Transform|TransformLocation (Transformation|GetActorTransform) (* DeltaSeconds (* (Variables|/Script/ProjectGroovy.KeyModeData|GetBPM (Variables|Default|GetmodeData)) (Variables|Default|GetbaseMovement)))) false false))))

(fn ConstructionScript)

(fn SetNoteKey
  (Variables|Default|SetnoteKey (Utilities|Array|Get(acopy) (Variables|Default|GetkeyArray) (Variables|Default|GetnoteIndex))))

(fn NoteScore
  (bind _noteindex (Variables|Default|GetnoteIndex))
  (bind _keyarray (Variables|Default|GetkeyArray))
  (bind _output (Utilities|Array|Get(acopy) _keyarray _noteindex))
  ;[0.15 0.15 0.15 0.5] Comes from the player class, which has read that the player has pressed a keyboard, so this method will see if it is relevant to this instance of the note, and what to do if it is.
  (Development|PrintString (Utilities|String|Append "Score note within measure " (Utilities|String|ToString(Integer) (Variables|Default|GetquarterBeat))))
  (if (or (Variables|Default|Getactive) (Variables|Default|GetbeingPlayed))
    (Development|PrintString "Hello")
    (bind _returnvalue (Actor|GetActorOfClass "/Game/Blueprints/Blueprints/main/BP_Player.BP_Player_C"))
    (Variables|Default|SetnoteKey _output)
    (if (Variables|Default|GetbeingPlayed)
      (Variables|Default|SetcollisionUsed (Variables|Default|Getnote_complete))
      (else
        (Variables|Default|SetcollisionUsed (Variables|Default|GetmainNote))))
    (bind (_array_element _array_index) (Utilities|Array|ForEachLoopwithBreak (Variables|Default|GetallNoteScoreActors) :!label _label)
      (:LoopBody
        (if (Collision|IsOverlappingActor (Variables|Default|GetcollisionUsed) _array_element :!class /Script/Engine.PrimitiveComponent)
          (Variables|Default|Setactive false)
          (bind _returnvalue_2 (Actor|GetActorOfClass "/Game/Widgets/main/RhythmHUD.RhythmHUD_C"))
          (if (Utilities|Enum|Equal(Enum) (Class|KismetInputLibrary|KeyGetDisplayName (Variables|/Game/Blueprints/Blueprints/main/BP_Player.BP_Player_C|GetkeyPressed _returnvalue) true) (Class|KismetInputLibrary|KeyGetDisplayName _output true))
            (Default|UpdateScore (Variables|/Game/Widgets/main/RhythmHUD.RhythmHUD_C|GetHUDRef _returnvalue_2) (Utilities|Array|Get(acopy) (Variables|Default|GetscoreMessages) _array_index) self (not (Variables|Default|GetbeingPlayed)))
            (if (and (Utilities|Enum|NotEqual(Enum) (Utilities|String|MakeLiteralString "Early") (Utilities|Array|Get(acopy) (Variables|Default|GetscoreMessages) _array_index)) (Utilities|Enum|NotEqual(Enum) (Utilities|String|MakeLiteralString "Late") (Utilities|Array|Get(acopy) (Variables|Default|GetscoreMessages) _array_index)))
              (Variables|Default|SetbeingPlayed (not (Variables|Default|GetbeingPlayed)))
              (goto _label Break)
              (else
                (goto _label Break)))
            (else
              (Default|UpdateScore (Variables|/Game/Widgets/main/RhythmHUD.RhythmHUD_C|GetHUDRef _returnvalue_2) "Wrong Note Played" self (not (Variables|Default|GetbeingPlayed)))
              (goto _label Break)))
          (else
            (Development|PrintString (Utilities|Array|Get(acopy) (Variables|Default|GetscoreMessages) _array_index))))))))