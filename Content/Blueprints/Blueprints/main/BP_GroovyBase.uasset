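; BP_GroovyBase is a Blueprint that assigns and preloads four danger sound cues, covering drain and wrong events for doll and audience.
; On BeginPlay it stores each sound in a variable and passes it to LoadSoundToMemory.
; That helper creates a 2D sound at zero volume and plays it immediately, a silent warm-up intended to get the audio into memory before it is needed.
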(event EventBeginPlay
  (bind _output_get (Variables|Default|SetdrainDollDanger "/Game/Audio/SND_weird_jingle.SND_weird_jingle"))
  (CallFunction|LoadSoundtoMemory _output_get)
  (bind _output_get_2 (Variables|Default|SetwrongAudienceDanger "/Game/Audio/SND_boo.SND_boo"))
  (CallFunction|LoadSoundtoMemory _output_get_2)
  (bind _output_get_3 (Variables|Default|SetdrainAudienceDanger "/Game/Audio/SND_horn.SND_horn"))
  (CallFunction|LoadSoundtoMemory _output_get_3)
  (bind _output_get_4 (Variables|Default|SetwrongDollDanger "/Game/Audio/SND_thx_scary.SND_thx_scary"))
  (CallFunction|LoadSoundtoMemory _output_get_4))

(event EventTick
  (params (DeltaSeconds :type Float%20%28single-precision%29)))

(fn ConstructionScript)

(fn LoadSoundtoMemory
  (params (newSound :type Sound%20Base%20Object%20Reference))
  (bind _returnvalue (Audio|CreateSound2D newSound 0.0 1.0 0.0 0))
  (Audio|Components|Audio|Play _returnvalue 0.0))