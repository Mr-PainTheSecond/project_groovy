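; BP_Beats is a moving beat marker in the rhythm game that drives song start and level completion.
; Once the audience initializes, it reads note pad settings, then moves at a BPM-scaled speed while unpaused in its associated game state.
; Overlapping a note calls its timing test; measure 24 starts or unpauses the song, and the final beat saves and opens the victory level.
; It destroys itself upon leaving the delete pad.
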(event Collision|EventActorEndOverlap
  (params (OtherActor :type Actor%20Object%20Reference))
  (Utilities|Casting|CastToBP_DeletePad OtherActor)
  (Actor|DestroyActor))

(event Collision|EventActorBeginOverlap
  (params (OtherActor :type Actor%20Object%20Reference))
  (bind _asbp_notes (Utilities|Casting|CastToBP_Notes OtherActor))
  (Class|NotePad|TestTime _asbp_notes)
  (if (not (< (Variables|Default|Getmeasure) 24))
    (if (== (Variables|Default|Getmeasure) 24)
      (if (Audio|Components|Audio|IsPlaying (Variables|/Script/ProjectGroovy.KeyModeData|Getsong (Variables|Default|GetmodeData)))
        (Class|KeyModeData|UnPauseAudio (Variables|Default|GetmodeData))
        (Development|PrintString "Unpausing...")
        (else
          (Development|PrintString "Starting Song")
          (Audio|Components|Audio|Play (Variables|/Script/ProjectGroovy.KeyModeData|Getsong (Variables|Default|GetmodeData)) 0.0)
          (Class|KeyModeData|UnPauseAudio (Variables|Default|GetmodeData))))
      (bind _returnvalue (Actor|GetActorOfClass "/Game/Blueprints/Blueprints/main/BP_RhythmGameMode.BP_RhythmGameMode_C"))
      (Variables|/Game/Blueprints/Blueprints/main/BP_RhythmGameMode.BP_RhythmGameMode_C|SetsongPlaying _returnvalue true)
      (else
        (bind _returnvalue_2 (Actor|GetActorOfClass "/Game/Blueprints/Blueprints/main/BP_RhythmGameMode.BP_RhythmGameMode_C"))
        (if (== (Variables|Default|Getmeasure) (Variables|/Game/Blueprints/Blueprints/main/BP_RhythmGameMode.BP_RhythmGameMode_C|GetfinalBeat _returnvalue_2))
          (bind _returnvalue_3 (SaveGame|CreateSaveGameObject "/Game/Blueprints/Blueprints/main/BP_SaveData.BP_SaveData_C"))
          (bind _returnvalue_4 (Actor|GetActorOfClass "/Game/Blueprints/Blueprints/main/BP_GroovyBase.BP_GroovyBase_C"))
          (bind _asbp_rhythm_game_mode (Utilities|Casting|CastToBP_RhythmGameMode (Game|GetGameMode)))
          (Class|ResultsSaveData|WriteandSave _returnvalue_3 _returnvalue_4 _asbp_rhythm_game_mode)
          (Game|OpenLevel(byObjectReference) "/Game/Maps/VictoryLevel.VictoryLevel"))))))

(event EventBeginPlay
  (bind _returnvalue (Actor|GetActorOfClass "/Game/Blueprints/Blueprints/main/BP_RhythmGameMode.BP_RhythmGameMode_C"))
  (Variables|Default|Setready (Variables|/Game/Blueprints/Blueprints/main/BP_RhythmGameMode.BP_RhythmGameMode_C|GetaudienceInitialized _returnvalue))
  (while (not (Variables|Default|Getready))
    (bind _returnvalue_2 (Actor|GetActorOfClass "/Game/Blueprints/Blueprints/main/BP_RhythmGameMode.BP_RhythmGameMode_C"))
    (Variables|Default|Setready (Variables|/Game/Blueprints/Blueprints/main/BP_RhythmGameMode.BP_RhythmGameMode_C|GetaudienceInitialized _returnvalue_2)))
  (bind _returnvalue_3 (Actor|GetActorOfClass "/Game/Blueprints/Blueprints/main/BP_NotePad.BP_NotePad_C"))
  (Variables|Default|SetbaseMovement (Variables|/Game/Blueprints/Blueprints/main/BP_NotePad.BP_NotePad_C|GetbaseMovement _returnvalue_3))
  (Variables|Default|SetBPM (Variables|/Game/Blueprints/Blueprints/main/BP_NotePad.BP_NotePad_C|GetBPM _returnvalue_3)))

(event EventTick
  (params (DeltaSeconds :type Float%20%28single-precision%29))
  (bind _returnvalue (Actor|GetActorOfClass "/Game/Blueprints/Blueprints/main/BP_GroovyBase.BP_GroovyBase_C"))
  (if (== (Variables|/Script/ProjectGroovy.ProjectGroovyBase|GetgameState _returnvalue) (Math|Conversions|ToInteger(Byte) (Variables|Default|GetassoicatedMode)))
    (bind _returnvalue_2 (Actor|GetActorOfClass "/Game/Blueprints/Blueprints/main/BP_Player.BP_Player_C"))
    (if (not (Variables|/Game/Blueprints/Blueprints/main/BP_Player.BP_Player_C|Getpaused _returnvalue_2))
      (Transformation|SetActorLocation (Math|Transform|TransformLocation (Transformation|GetActorTransform) (* DeltaSeconds (* (Variables|/Script/ProjectGroovy.KeyModeData|GetBPM (Variables|Default|GetmodeData)) (Variables|Default|GetbaseMovement)))) false false))))

(fn ConstructionScript)